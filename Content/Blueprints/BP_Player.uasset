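; Player Blueprint that displays its local network role, health and rocket count through a WBP_Role widget held by its UI component.
; BeginPlay writes the role text, while the health and rocket-count change events push new values through two setter functions.
; For debugging, F calls a health-decrease cheat and Tick prints the name of each valid rocket in RocketInstances, whose only Add node here is unwired.
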(event `self.ReceiveTick`
  (params (DeltaSeconds :type "Float (single-precision)"))
  (for _array_element (`self.RocketInstances`)
    (if (`KismetSystemLibrary.IsValid` _array_element)
      (`KismetSystemLibrary.PrintString` (`KismetSystemLibrary.GetObjectName` _array_element)))))

(event `self.ReceiveBeginPlay`
  (bind _aswbp_role (cast `/Game/Blueprints/UI/WBP_Role` (`WidgetComponent.GetUserWidgetObject` (`self.UI`))))
  (`/Game/Blueprints/UI/WBP_Role.SetLocalText` _aswbp_role (`KismetTextLibrary.Conv_StringToText` (`|GetEnumeratorNameAsString` (`self.GetLocalRole`)))))

(event `self.BP_OnNumRocketsChanged`
  (params (NewNumRockets :type Integer))
  (`self.SetNumRocketsInWidget` NewNumRockets))

(event `self.BP_OnHealthChanged`
  (params (NewHealth :type "Float (single-precision)"))
  (`self.SetHealthInWidget` NewHealth))

(event `Key|F`
  (params (Key :type "Key Structure"))
  (:`Pressed`
    (`self.Cheat_DecreaseHealthOnPlayer`)))

(fn `SetHealthInWidget`
  (params (InHealth :type "Float (double-precision)"))
  (bind _aswbp_role (cast `/Game/Blueprints/UI/WBP_Role` (`WidgetComponent.GetUserWidgetObject` (`self.UI`))))
  (`/Game/Blueprints/UI/WBP_Role.SetHealth` _aswbp_role InHealth))

(fn `SetNumRocketsInWidget`
  (params (`In Num Rockets` :type Integer))
  (bind _aswbp_role (cast `/Game/Blueprints/UI/WBP_Role` (`WidgetComponent.GetUserWidgetObject` (`self.UI`))))
  (`/Game/Blueprints/UI/WBP_Role.Set Num Rockets` _aswbp_role `In Num Rockets`))

(fn `UserConstructionScript`)